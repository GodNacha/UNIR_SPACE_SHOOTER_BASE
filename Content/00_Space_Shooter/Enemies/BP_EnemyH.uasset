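; BP_EnemyH is a space shooter enemy that moves along its right vector, building on a parent class's behavior.
; On BeginPlay it sets MovementVector from the actor's right vector.
; Overlapping an actor tagged "Lateral" reverses that vector and shortens DelayShoot, with a small floor on the delay, so each bounce tightens the shooting interval.
; Movement and shooting are not implemented in this graph, and its Tick is disabled.
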(event `self.ReceiveBeginPlay`
  (`parent.ReceiveBeginPlay`)
  (set `self.MovementVector` (`self.GetActorRightVector`)))

(event `self.ReceiveActorBeginOverlap`
  (params (OtherActor :type "Actor Object Reference"))
  (bind _returnvalue (- (`self.DelayShoot`) 0.1))
  (`parent.ReceiveActorBeginOverlap` OtherActor)
  (if (`KismetArrayLibrary.Array_Contains` (`Actor.Tags` OtherActor) "Lateral")
    (set `self.MovementVector` (* (`self.MovementVector`) (-1.0 -1.0 -1.0)))
    (set `self.DelayShoot` _returnvalue)
    (if (< _returnvalue 0.0)
      (set `self.DelayShoot` 0.1))))

(fn `UserConstructionScript`
  (`parent.UserConstructionScript`))